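; BP_RCupboard is an interactable cupboard whose static mesh slides back and forth along its relative X axis.
; EmptyHandInteract plays a door sound at world origin, then plays or reverses a Timeline according to State.
; The Timeline track drives the mesh position, and finishing toggles State.
; AnimationEnd gates interaction, but only the forward branch clears it, so reversing leaves interaction unlocked.
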(event `/Game/BluePrints/EmptyHandInterface.Empty Hand Interact`
  (bind _animation_end (`self.animation end`))
  (if _animation_end
    (`GameplayStatics.PlaySoundAtLocation` "/Game/BluePrints/Sounds/DoorOpen_Cue.DoorOpen_Cue" (0.0 0.0 0.0) (struct) 1.0 1.0 0.0 null null null null)
    (if (`self.state`)
      (set `self.animation end` false)
      (bind (_direction _newtrack_0) (`Timeline|Timeline` :!label _label)
        (:`Update`
          (`SceneComponent.K2_SetRelativeLocation` (`self.StaticMesh`) (`KismetMathLibrary.MakeVector` _newtrack_0) false false))
        (:`Finished`
          (set `self.animation end` true)
          (set `self.state` (xor (`self.state`) true))))
      (else
        (set `self.animation end` _animation_end)
        (goto _label :!via `Reverse`)))))

(fn `UserConstructionScript`)