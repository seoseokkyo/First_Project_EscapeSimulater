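; BP_Door is a lockable door that the player unlocks with a key and then opens and closes by hand.
; PlaceInteract accepts a held BP_DoorKey, sets Open, destroys the key, resets the player's hand state and plays a success sound.
; EmptyHandInteract toggles an unlocked door, playing or reversing a timeline that drives its yaw.
; Unlocking, or trying a locked door, shows a temporary UI_Message popup in Korean.
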(event `/Game/BluePrints/PlaceInterface.PlaceInteract`
  (params (TryInteractActor :type "Actor Object Reference"))
  ;[1 1 1] 상호작용을 시도하는 (플레이어의 손에 있는)객체가 열쇠인지 확인
  (bind _asbp_door_key (cast `/Game/BluePrints/BP_Door/BP_DoorKey` TryInteractActor))
  (set `self.As BP Door Key` _asbp_door_key)
  ;[1 1 1] 열쇠 확인 시 DoorOpen
  (set `self.Open` true)
  ;[1 1 1] 플레이어 캐릭터에서 상호작용을 완료한 액터 삭제 및 State변경(다른 상호작용이 정상동작하도록)
  (bind _asbp_player (cast `/Game/BluePrints/BP_Player` (`GameplayStatics.GetPlayerCharacter` 0)))
  (set `/Game/BluePrints/BP_Player.EmptyHand` true _asbp_player)
  (set `/Game/BluePrints/BP_Player.HandlingObject` null _asbp_player)
  (`self.K2_DestroyActor` (`self.As BP Door Key`))
  ;[1 1 1] 성공효과음
  (`GameplayStatics.PlaySoundAtLocation` "/Game/BluePrints/Sounds/Succesed__Cue.Succesed__Cue" (0.0 0.0 0.0) (struct) 1.0 1.0 0.0 null null null null)
  ;[1 1 1] Message 팝업 (문이 열렸습니다.)
  (bind _returnvalue (`|CreateWidget` "/Game/BluePrints/UI_Notifications/UI_Message.UI_Message_C"))
  (bind _output_get (set `self.Message` _returnvalue))
  (`UserWidget.AddToViewport` _output_get 0)
  (`/Game/BluePrints/UI_Notifications/UI_Message.Set Text` _output_get "문이 열렸습니다.")
  (`KismetSystemLibrary.Delay` 2.0)
  (`Widget.RemoveFromParent` _output_get))

(event `/Game/BluePrints/EmptyHandInterface.Empty Hand Interact`
  ;[1 1 1] 빈손으로 상호작용 시도 시 잠금이 해제된 상태인지 확인
  (if (`self.Open`)
    ;[1 1 1] 매 회 Open Close 변경
    (bind _output_get (set `self.State` (xor (`self.State`) true)))
    ;[1 1 1] Animation
    (if _output_get
      (`GameplayStatics.PlaySoundAtLocation` "/Game/BluePrints/Sounds/DoorOpen_Cue.DoorOpen_Cue" (0.0 0.0 0.0) (struct) 1.0 1.0 0.0 null null null null)
      (bind (_direction _door_rotating) (`Timeline|Timeline_0` :!label _label)
        (:`Update`
          (`SceneComponent.K2_SetRelativeRotation` (`self.Door`) (`KismetMathLibrary.MakeRotator` 0.0 0.0 _door_rotating) false false)))
      (else
        (`GameplayStatics.PlaySoundAtLocation` "/Game/BluePrints/Sounds/DoorOpen_Cue.DoorOpen_Cue" (0.0 0.0 0.0) (struct) 1.0 1.0 0.0 null null null null)
        (goto _label :!via `Reverse`)))
    (else
      ;[1 1 1] Message 팝업 (문이 잠겨있습니다.)
      (bind _returnvalue (`|CreateWidget` "/Game/BluePrints/UI_Notifications/UI_Message.UI_Message_C"))
      (bind _output_get_2 (set `self.Message` _returnvalue))
      (`UserWidget.AddToViewport` _output_get_2 0)
      (`/Game/BluePrints/UI_Notifications/UI_Message.Set Text` _output_get_2 "문이 잠겨있습니다.")
      (`KismetSystemLibrary.Delay` 2.0)
      (`Widget.RemoveFromParent` _output_get_2))))

(fn `UserConstructionScript`)