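; BP_DoorKey is a door key pickup that marks the player as holding a key through inspect events.
; InspectStart sets HasKey, attaches the key to the player's Item component with physics and collision off, and shows a timed Korean "key acquired" message.
; InspectEnd detaches it and restores physics and collision, but still sets HasKey true.
; The Sphere overlap event is empty, leaving older overlap-pickup logic unconnected.
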(event `self.Sphere.OnComponentBeginOverlap`
  (params (OverlappedComponent :type "PrimitiveComponent Object Reference") (OtherActor :type "Actor Object Reference") (OtherComp :type "PrimitiveComponent Object Reference") (OtherBodyIndex :type Integer) (bFromSweep :type Boolean) (SweepResult :type "HitResult Structure (by ref)"))
  ;[1 1 1] Player 가 열쇠에 다가갔을 때 열쇠 사라짐 + "열쇠를 획득했습니다." 출력
)

(event `/Game/BluePrints/InspectInteract.Inspect Start`
  (params (BP_Player :type "/Game/BluePrints/BP_Player Object Reference"))
  (bind _door_key (`self.Door_Key`))
  (bind _asbp_player (cast `/Game/BluePrints/BP_Player` BP_Player))
  (bind _output_get (set `self.Player` _asbp_player))
  (set `/Game/BluePrints/BP_Player.HasKey?` true _output_get)
  (`self.EnableInput` (`GameplayStatics.GetPlayerController` 0))
  (`self.K2_AttachToComponent` (`/Game/BluePrints/BP_Player.Item` (`self.Player`)) "None" "SnapToTarget" "SnapToTarget" "KeepRelative")
  (`PrimitiveComponent.SetSimulatePhysics` _door_key false)
  (`PrimitiveComponent.SetCollisionEnabled` _door_key "NoCollision")
  (set `/Game/BluePrints/BP_Player.HandlingObject` null (`self.Player`))
  (`self.K2_SetActorRelativeRotation` (struct :`Pitch` 90.0))
  (bind _returnvalue (`|CreateWidget` "/Game/BluePrints/UI_Notifications/UI_Message.UI_Message_C"))
  (bind _output_get_2 (set `self.Message` _returnvalue))
  (`UserWidget.AddToViewport` _output_get_2 0)
  (`/Game/BluePrints/UI_Notifications/UI_Message.Set Text` _output_get_2 "열쇠를 획득했습니다.")
  (`KismetSystemLibrary.Delay` 3.0)
  (`Widget.RemoveFromParent` _output_get_2))

(event `/Game/BluePrints/InspectInteract.Inspect End`
  (params (BP_Player :type "/Game/BluePrints/BP_Player Object Reference"))
  (bind _door_key (`self.Door_Key`))
  (bind _asbp_player (cast `/Game/BluePrints/BP_Player` BP_Player))
  (bind _output_get (set `self.Player` _asbp_player))
  (set `/Game/BluePrints/BP_Player.HasKey?` true _output_get)
  (`self.DisableInput` (`GameplayStatics.GetPlayerController` 0))
  (`self.K2_SetActorRelativeLocation` (0.0 0.0 0.0))
  (`self.K2_DetachFromActor` "KeepWorld" "KeepWorld")
  (`PrimitiveComponent.SetSimulatePhysics` _door_key true)
  (`PrimitiveComponent.SetCollisionEnabled` _door_key "QueryAndPhysics"))

(fn `UserConstructionScript`)