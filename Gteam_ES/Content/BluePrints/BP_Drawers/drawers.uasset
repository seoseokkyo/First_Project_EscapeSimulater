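; Drawer Blueprint that toggles its own player input through two overlap volumes, Drawer_Box and Drawer_open.
; Begin overlap enables input only when the other actor is itself a drawers, while end overlap disables it for BP_Player.
; Drawer_Box passes the overlap body index as the player index, whereas Drawer_open uses player zero.
; The graph contains no input handling or drawer movement.
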(event `self.Drawer_Box.OnComponentBeginOverlap`
  (params (OverlappedComponent :type "PrimitiveComponent Object Reference") (OtherActor :type "Actor Object Reference") (OtherComp :type "PrimitiveComponent Object Reference") (OtherBodyIndex :type Integer) (bFromSweep :type Boolean) (SweepResult :type "HitResult Structure (by ref)"))
  (cast `/Game/BluePrints/BP_Drawers/drawers` OtherActor)
  (`self.EnableInput` (`GameplayStatics.GetPlayerController` OtherBodyIndex)))

(event `self.Drawer_Box.OnComponentEndOverlap`
  (params (OverlappedComponent :type "PrimitiveComponent Object Reference") (OtherActor :type "Actor Object Reference") (OtherComp :type "PrimitiveComponent Object Reference") (OtherBodyIndex :type Integer))
  (cast `/Game/BluePrints/BP_Player` OtherActor)
  (`self.DisableInput` (`GameplayStatics.GetPlayerController` (stale `self.Drawer_Box.OnComponentBeginOverlap` OtherBodyIndex))))

(event `self.Drawer_open.OnComponentBeginOverlap`
  (params (OverlappedComponent :type "PrimitiveComponent Object Reference") (OtherActor :type "Actor Object Reference") (OtherComp :type "PrimitiveComponent Object Reference") (OtherBodyIndex :type Integer) (bFromSweep :type Boolean) (SweepResult :type "HitResult Structure (by ref)"))
  (cast `/Game/BluePrints/BP_Drawers/drawers` OtherActor)
  (`self.EnableInput` (`GameplayStatics.GetPlayerController` 0)))

(event `self.Drawer_open.OnComponentEndOverlap`
  (params (OverlappedComponent :type "PrimitiveComponent Object Reference") (OtherActor :type "Actor Object Reference") (OtherComp :type "PrimitiveComponent Object Reference") (OtherBodyIndex :type Integer))
  (cast `/Game/BluePrints/BP_Player` OtherActor)
  (`self.DisableInput` (`GameplayStatics.GetPlayerController` 0)))

(fn `UserConstructionScript`)