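; BP_GameState is a game state Blueprint that reacts to completion of three puzzles.
; Tick polls the TargetSolved flags and clears each one when set.
; For puzzle 1, it finds BP_DoorKey, makes it visible, sets its collision profile, calls PuzzleSolved on BP_PuzzleSolved and shows a two-second UI_Message.
; Puzzles 2 and 3 only reset their flags, with completion effects left for later.
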(event `self.ReceiveTick`
  (params (DeltaSeconds :type "Float (single-precision)"))
  (`|ExecutionSequence`
    (:`then_0`
      ;[1 1 1] 1번 퍼즐 완료체크 및 플래그 해제
      (if (`self.TargetSolved_1`)
        (set `self.TargetSolved_1` false)
        ;[1 1 1] 퍼즐 풀리면 열쇠 나오면서 팡파레효과
        (bind _returnvalue (`GameplayStatics.GetActorOfClass` "/Game/BluePrints/BP_Door/BP_DoorKey.BP_DoorKey_C"))
        (`/Engine/EditorBlueprintResources/StandardMacros.IsValid` _returnvalue
          (:`Is Valid`
            (`SceneComponent.SetVisibility` (`Actor.RootComponent` _returnvalue) true true)
            (`PrimitiveComponent.SetCollisionProfileName` (`/Game/BluePrints/BP_Door/BP_DoorKey.Door_Key` _returnvalue) "Collision" false)
            (bind _returnvalue_2 (`GameplayStatics.GetActorOfClass` "/Game/Puzzle/SuccesedEffect/BP_PuzzleSolved.BP_PuzzleSolved_C"))
            (bind _asbp_puzzle_solved (cast `/Game/Puzzle/SuccesedEffect/BP_PuzzleSolved` _returnvalue_2))
            (`/Game/Puzzle/SuccesedEffect/BP_PuzzleSolved.PuzzleSolved ` _asbp_puzzle_solved)
            ;[1 1 1] 퍼즐을 풀었습니다! UI 출력
            (bind _returnvalue_3 (`|CreateWidget` "/Game/BluePrints/UI_Notifications/UI_Message.UI_Message_C" (`GameplayStatics.GetPlayerController` 0)))
            (`/Game/BluePrints/UI_Notifications/UI_Message.Set Text` _returnvalue_3 "퍼즐을 풀었습니다.")
            (`UserWidget.AddToViewport` _returnvalue_3 0)
            (`KismetSystemLibrary.Delay` 2.0)
            (`Widget.RemoveFromParent` _returnvalue_3)))))
    (:`then_1`
      ;[1 1 1] 2번퍼즐 완료체크 및 플래그 해제(이후 완료 이펙트 필요 시 작업)
      (if (`self.TargetSolved_2`)
        (set `self.TargetSolved_2` false)))
    (:`then_2`
      ;[1 1 1] 3번퍼즐 완료체크 및 플래그 해제(이후 완료 이펙트 필요 시 작업)
      (if (`self.TargetSolved_3`)
        (set `self.TargetSolved_3` false)))))

(fn `UserConstructionScript`)