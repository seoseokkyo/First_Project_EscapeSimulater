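; BP_GearHandle is a pickup actor for a gear handle, apparently part of the gear toy.
; An empty-hand interaction or an OnReleased event on SM_GearHandle triggers the same logic, duplicated in both handlers.
; It casts player character 0 to BP_Player and, if HaveHandle is false, sets it to true and destroys itself.
; BeginPlay, overlap, Tick and the construction script are empty.
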(event `/Game/BluePrints/EmptyHandInterface.Empty Hand Interact`
  (bind _asbp_player (cast `/Game/BluePrints/BP_Player` (`GameplayStatics.GetPlayerCharacter` 0)))
  (if (not (`/Game/BluePrints/BP_Player.haveHandle` _asbp_player))
    (set `/Game/BluePrints/BP_Player.haveHandle` true _asbp_player)
    (`self.K2_DestroyActor`)))

(event `self.SM_GearHandle.OnReleased`
  (params (TouchedComponent :type "PrimitiveComponent Object Reference") (ButtonReleased :type "Key Structure"))
  (bind _asbp_player (cast `/Game/BluePrints/BP_Player` (`GameplayStatics.GetPlayerCharacter` 0)))
  (if (not (`/Game/BluePrints/BP_Player.haveHandle` _asbp_player))
    (set `/Game/BluePrints/BP_Player.haveHandle` true _asbp_player)
    (`self.K2_DestroyActor`)))

(fn `UserConstructionScript`)