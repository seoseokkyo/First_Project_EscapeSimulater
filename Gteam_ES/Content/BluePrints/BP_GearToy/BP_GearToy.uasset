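; BP_GearToy is a puzzle toy with two handle-locked doors and a button that pops up a hint panel.
; Each slot consumes the player's handle, spawns a BP_GearHandle, rotates it by timeline, then swings its door open.
; The switch door requires the handle door to be open first.
; The button's chained timelines end by setting TargetSolved3 in BP_GameState, resetting player interaction state and destroying both handles and the toy.
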(event `self.SM_HandleSlot_Handle.OnReleased`
  (params (TouchedComponent :type "PrimitiveComponent Object Reference") (ButtonReleased :type "Key Structure"))
  ;[1 1 1] 핸들이 있는 도어를 열기위한 핸들슬롯 (맵상에 있는 핸들을 찾아 와야 동작이 됨)
  (bind _asbp_player (cast `/Game/BluePrints/BP_Player` (`GameplayStatics.GetPlayerCharacter` 0)))
  (if (`/Game/BluePrints/BP_Player.haveHandle` _asbp_player)
    (if (not (`self.HandleDoorOpen`))
      (`/Game/BluePrints/BP_Player.SetHaveHandle` _asbp_player false)
      (bind _returnvalue (`|SpawnActorFromClass` "/Game/BluePrints/BP_GearToy/BP_GearHandle.BP_GearHandle_C" (`SceneComponent.K2_GetComponentToWorld` (`self.HandleSlot_HandleDoor`)) "Undefined" "MultiplyWithRoot" null null))
      (bind _output_get (set `self.GearHandle` _returnvalue))
      (`self.K2_AttachToComponent` _output_get (`self.HandleSlot_HandleDoor`) "None" "SnapToTarget" "SnapToTarget" "KeepRelative" true)
      (`PrimitiveComponent.SetCollisionEnabled` (`/Game/BluePrints/BP_GearToy/BP_GearHandle.SM_GearHandle` _returnvalue) "NoCollision")
      (`GameplayStatics.PlaySoundAtLocation` "/Game/BluePrints/Sounds/GearToy/GearToyHandleRotate_Cue.GearToyHandleRotate_Cue" (0.0 0.0 0.0) (struct) 1.0 1.0 0.0 null null null null)
      (bind (_direction `_새_트랙_0`) (`Timeline|타임라인`)
        (:`Update`
          (`self.K2_SetActorRelativeRotation` _returnvalue (`KismetMathLibrary.MakeRotator` `_새_트랙_0`) false false))
        (:`Finished`
          (set `self.HandleDoorOpen` true)
          (`GameplayStatics.PlaySoundAtLocation` "/Game/BluePrints/Sounds/GearToy/UnLock_Cue.UnLock_Cue" (0.0 0.0 0.0) (struct) 1.0 1.0 0.0 null null null null)
          (bind (_direction_2 _dooropen) (`Timeline|HandleDoor Open`)
            (:`Update`
              (`SceneComponent.K2_SetRelativeRotation` (`self.SM_GearToyDoor_Handle`) (`KismetMathLibrary.MakeRotator` _dooropen) false false))))))))

(event `self.SM_HandleSlot_Switch.OnReleased`
  (params (TouchedComponent :type "PrimitiveComponent Object Reference") (ButtonReleased :type "Key Structure"))
  ;[1 1 1] 스위치가 있는 도어를 열기위한 핸들슬롯 (핸들이 있는 슬롯이 열렸고, 해당 핸들을 주워야 동작이 됨)
  (bind _asbp_player (cast `/Game/BluePrints/BP_Player` (`GameplayStatics.GetPlayerCharacter` 0)))
  (if (`/Game/BluePrints/BP_Player.haveHandle` _asbp_player)
    (if (`self.HandleDoorOpen`)
      (`/Game/BluePrints/BP_Player.SetHaveHandle` _asbp_player false)
      (bind _returnvalue (`|SpawnActorFromClass` "/Game/BluePrints/BP_GearToy/BP_GearHandle.BP_GearHandle_C" (`SceneComponent.K2_GetComponentToWorld` (`self.HandleSlot_Switch`)) "Undefined" "MultiplyWithRoot" null null))
      (bind _output_get (set `self.GearHandle2` _returnvalue))
      (`self.K2_AttachToComponent` _output_get (`self.HandleSlot_Switch`) "None" "SnapToTarget" "SnapToTarget" "KeepRelative" true)
      (`PrimitiveComponent.SetCollisionEnabled` (`/Game/BluePrints/BP_GearToy/BP_GearHandle.SM_GearHandle` _returnvalue) "NoCollision")
      (`GameplayStatics.PlaySoundAtLocation` "/Game/BluePrints/Sounds/GearToy/GearToyHandleRotate_Cue.GearToyHandleRotate_Cue" (0.0 0.0 0.0) (struct) 1.0 1.0 0.0 null null null null)
      (bind (_direction `_새_트랙_0`) (`Timeline|타임라인_1`)
        (:`Update`
          (`self.K2_SetActorRelativeRotation` _returnvalue (`KismetMathLibrary.MakeRotator` `_새_트랙_0`) false false))
        (:`Finished`
          (`GameplayStatics.PlaySoundAtLocation` "/Game/BluePrints/Sounds/GearToy/UnLock_Cue.UnLock_Cue" (0.0 0.0 0.0) (struct) 1.0 1.0 0.0 null null null null)
          (bind (_direction_2 _switchdooropen) (`Timeline|타임라인_0`)
            (:`Update`
              (`SceneComponent.K2_SetRelativeRotation` (`self.SM_GearToyDoorSwitch`) (`KismetMathLibrary.MakeRotator` _switchdooropen 0.0 180.0) false false))))))))

(event `self.GearToyButton.OnReleased`
  (params (TouchedComponent :type "PrimitiveComponent Object Reference") (ButtonReleased :type "Key Structure"))
  ;[1 1 1] 힌트가 적힌 패널을 팝업시키기 위한 스위치
  (`GameplayStatics.PlaySoundAtLocation` "/Game/BluePrints/Sounds/StrongBox/ButtonPress_Cue.ButtonPress_Cue" (0.0 0.0 0.0) (struct) 1.0 1.0 0.0 null null null null)
  (bind (_direction `_새_트랙_0`) (`Timeline|ButtonPush`)
    (:`Update`
      (`SceneComponent.K2_SetRelativeLocation` (`self.GearToyButton`) (`KismetMathLibrary.MakeVector` 0.0 (+ `_새_트랙_0` -8.4) 3.0) false false))
    (:`Finished`
      (`GameplayStatics.PlaySoundAtLocation` "/Game/BluePrints/Sounds/GearToy/HintPop_Cue.HintPop_Cue" (0.0 0.0 0.0) (struct) 1.0 1.0 0.0 null null null null)
      (bind (_direction_2 `_새_트랙_0_2`) (`Timeline|HintPopup`)
        (:`Update`
          (`SceneComponent.K2_SetRelativeLocation` (`self.SM_GearToyHint`) (`KismetMathLibrary.MakeVector` 0.0 0.0 (+ `_새_트랙_0_2` 5.0)) false false))
        (:`Finished`
          (`self.RotateOff`)
          (bind _asbp_game_state (cast `/Game/BluePrints/BP_GameState` (`GameplayStatics.GetGameState`)))
          (set `/Game/BluePrints/BP_GameState.TargetSolved_3` true _asbp_game_state)
          (bind _asbp_player (cast `/Game/BluePrints/BP_Player` (`GameplayStatics.GetPlayerCharacter` 0)))
          (`/Game/BluePrints/BP_Player.Call Toggle Cursor` _asbp_player)
          (set `/Game/BluePrints/BP_Player.CorrectActor` null _asbp_player)
          (set `/Game/BluePrints/BP_Player.EmptyHand` true _asbp_player)
          (`self.K2_DestroyActor` (`self.GearHandle`))
          (`self.K2_DestroyActor` (`self.GearHandle2`))
          (`self.K2_DestroyActor`))))))

(fn `UserConstructionScript`)