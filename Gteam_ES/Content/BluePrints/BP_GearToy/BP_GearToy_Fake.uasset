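; Decoy gear toy that hands the player the real BP_GearToy when inspected.
; On BeginPlay it finds the real toy; InspectStart swaps their locations, attaches the real one to the player's ItemPosition as the held object, and disables its own InspectMesh physics and collision.
; SwapFakeToy&ReleaseHand detaches both actors, swaps their locations again and restores the fake's physics and collision.
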(event `self.ReceiveBeginPlay`
  (bind _returnvalue (`GameplayStatics.GetActorOfClass` "/Game/BluePrints/BP_GearToy/BP_GearToy.BP_GearToy_C"))
  (set `self.RealGearToy` _returnvalue))

(event `/Game/BluePrints/InspectInteract.Inspect Start`
  (params (BP_Player :type "/Game/BluePrints/BP_Player Object Reference"))
  (bind _inspectmesh (`self.InspectMesh`))
  ;[1 1 1] Inspect Start 이벤트가 실행될 시 self를 Player의 Item Position 컴포넌트에 부착
  (bind _output_get (set `self.Player` BP_Player))
  (bind _output_get_2 (set `/Game/BluePrints/BP_Player.CorrectActor` (`self.RealGearToy`) _output_get))
  (set `/Game/BluePrints/BP_Player.HandlingObject` _output_get_2 _output_get)
  (set `/Game/BluePrints/BP_Player.EmptyHand` false _output_get)
  (set `self.TempLocation` (`self.K2_GetActorLocation` (`self.RealGearToy`)))
  (`self.K2_SetActorLocation` (`self.RealGearToy`) (`self.K2_GetActorLocation` self) false false)
  (`self.K2_SetActorLocation` self (`self.TempLocation`) false false)
  (`self.K2_AttachToComponent` (`self.RealGearToy`) (`/Game/BluePrints/BP_Player.ItemPosition` (`self.Player`)) "None" "SnapToTarget" "SnapToTarget" "KeepRelative" true)
  (`GameplayStatics.PlaySoundAtLocation` "/Game/BluePrints/Sounds/GetItem_Cue.GetItem_Cue" (0.0 0.0 0.0) (struct) 1.0 1.0 0.0 null null null null)
  ;[1 1 1] Inspect Mesh의 피직스 시뮬레이트를 종료하고 콜리전 설정을 변경함
  (`PrimitiveComponent.SetSimulatePhysics` _inspectmesh false)
  (`PrimitiveComponent.SetCollisionEnabled` _inspectmesh "NoCollision")
  ;[1 1 1] self의 각도를 변경함
  (`self.K2_SetActorRelativeRotation` (struct)))

(event `SwapFakeToy&ReleaseHand`
  (bind _inspectmesh (`self.InspectMesh`))
  (`self.K2_DetachFromActor` (`self.RealGearToy`) "KeepWorld" "KeepWorld" "KeepRelative")
  (`self.K2_DetachFromActor` "KeepWorld" "KeepWorld")
  (set `self.TempLocation` (`self.K2_GetActorLocation` (`self.RealGearToy`)))
  (`self.K2_SetActorLocation` (`self.RealGearToy`) (`self.K2_GetActorLocation` self) false false)
  (`self.K2_SetActorLocation` self (`self.TempLocation`) false false)
  (`PrimitiveComponent.SetSimulatePhysics` _inspectmesh true)
  (`PrimitiveComponent.SetCollisionEnabled` _inspectmesh "QueryAndPhysics"))

(event `/Game/BluePrints/InspectInteract.Inspect End`
  (params (BP_Player :type "/Game/BluePrints/BP_Player Object Reference")))

(fn `UserConstructionScript`)