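; BP_Body is the head statue body that runs a button puzzle where buttons 1, 3 and 6 form the correct answer.
; On BeginPlay it caches those three child-actor buttons, and ButtonPressed counts each press.
; From the third press, CompleteCheck sets TargetSolved2 on BP_GameState if all three are pressed.
; Otherwise it zeroes the count and fires StatueButtonReset.
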(event `self.ReceiveBeginPlay`
  ;[1 1 1] Button1,3,6 데이터를 받아옴
  (bind _asbp_button_1_a (cast `/Game/BluePrints/BP_HeadStatue/BP_Button/BP_Button1_a` (`ChildActorComponent.ChildActor` (`self.BP_Button1`))))
  (set `self.As BP Button 1 A` _asbp_button_1_a)
  (bind _asbp_button_3_a (cast `/Game/BluePrints/BP_HeadStatue/BP_Button/BP_Button3_a` (`ChildActorComponent.ChildActor` (`self.BP_Button3`))))
  (set `self.As BP Button 3 A` _asbp_button_3_a)
  (bind _asbp_button_6_a (cast `/Game/BluePrints/BP_HeadStatue/BP_Button/BP_Button6_a` (`ChildActorComponent.ChildActor` (`self.BP_Button6`))))
  (set `self.As BP Button 6 A` _asbp_button_6_a))

(event `ThreeButtonPresseCheck`
  (if (>= (`self.ButtonPressCount`) 3)
    (bind _complete (`self.Complete Check`))
    (if (not _complete)
      (set `self.ButtonPressCount` 0)
      (`self.StatueButtonReset`))))

(fn `ButtonPressed`
  (`/Engine/EditorBlueprintResources/StandardMacros.IncrementInt` (`self.ButtonPressCount`)
    (:`  `
      (`self.ThreeButtonPresseCheck`))))

(fn `Complete Check`
  (returns (Complete :type Boolean))
  ;[1 1 1] Button 1,3,6 의 Is Pressed True 값 모두 받아왔는지 확인
  (if (`/Game/BluePrints/BP_HeadStatue/BP_Button/BP_Button1_a.Is Pressed` (`self.As BP Button 1 A`))
    (if (`/Game/BluePrints/BP_HeadStatue/BP_Button/BP_Button3_a.Is Pressed` (`self.As BP Button 3 A`))
      (if (`/Game/BluePrints/BP_HeadStatue/BP_Button/BP_Button6_a.Is Pressed` (`self.As BP Button 6 A`))
        ;[1 1 1] 성공시 Gamestate - Target Solved2 에 저장
        (bind _asbp_game_state (cast `/Game/BluePrints/BP_GameState` (`GameplayStatics.GetGameState`)))
        (bind _output_get (set `/Game/BluePrints/BP_GameState.TargetSolved_2` true _asbp_game_state))
        (return _output_get)
        (else
          _))))
  (return false))

(fn `UserConstructionScript`)