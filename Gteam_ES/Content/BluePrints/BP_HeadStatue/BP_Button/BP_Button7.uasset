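; BP_Button7 is one of the pressable buttons on the head statue, expected to live as a child actor of BP_Body.
; An empty-hand interaction plays a timeline that moves Part7 along Z, then sets IsPressed and notifies BP_Body through ButtonPressed.
; On BeginPlay it binds to the body's StatueButtonReset event, which plays a second timeline on a pressed button and clears the flag when finished.
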(event `self.Empty Hand Interact`
  ;[1 1 1] 클릭시 버튼 눌림
  (bind (_direction _part1pressed) (`Timeline|Timeline` :!via `PlayFromStart`)
    (:`Update`
      (`SceneComponent.K2_SetRelativeLocation` (`self.Part7`) (`KismetMathLibrary.MakeVector` 0.0 0.0 _part1pressed) false false))
    (:`Finished`
      (set `self.Is Pressed` true)
      (bind _asbp_body (cast `/Game/BluePrints/BP_HeadStatue/BP_Button/BP_Body` (`self.GetParentActor`)))
      (`/Game/BluePrints/BP_HeadStatue/BP_Button/BP_Body.ButtonPressed` _asbp_body))))

(event `self.ReceiveBeginPlay`
  (bind _asbp_body (cast `/Game/BluePrints/BP_HeadStatue/BP_Button/BP_Body` (`self.GetParentActor`)))
  (add `/Game/BluePrints/BP_HeadStatue/BP_Button/BP_Body.StatueButtonReset` _asbp_body (delegate `ButtonReset`)))

(event `ButtonReset`
  (if (`self.Is Pressed`)
    (bind (_direction _part1pressed) (`Timeline|Timeline_0` :!via `PlayFromStart`)
      (:`Update`
        (`SceneComponent.K2_SetRelativeLocation` (`self.Part7`) (`KismetMathLibrary.MakeVector` 0.0 0.0 _part1pressed) false false))
      (:`Finished`
        (set `self.Is Pressed` false)))))

(fn `UserConstructionScript`)