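; BP_HintPaper is a hint paper, initially stuck to a wall, that the player picks up to inspect.
; InspectStart enables input, plays the item sound, snaps the actor to the player's ItemPosition and registers it as HandlingObject.
; It disables mesh physics and collision for the attach, then re-enables physics so the paper no longer stays on the wall.
; InspectEnd disables input, detaches the actor and restores physics and collision.
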(event `self.Inspect Start`
  (params (BP_Player :type "/Game/BluePrints/BP_Player Object Reference"))
  (bind _staticmesh1 (`self.StaticMesh1`))
  (set `self.Player` BP_Player)
  (`self.EnableInput` (`GameplayStatics.GetPlayerController` 0))
  (`self.K2_AttachToComponent` (`/Game/BluePrints/BP_Player.ItemPosition` (`self.Player`)) "None" "SnapToTarget" "SnapToTarget" "KeepRelative")
  (`GameplayStatics.PlaySoundAtLocation` "/Game/BluePrints/Sounds/GetItem_Cue.GetItem_Cue" (0.0 0.0 0.0) (struct) 1.0 1.0 0.0 null null null null)
  (`PrimitiveComponent.SetSimulatePhysics` _staticmesh1 false)
  (`PrimitiveComponent.SetCollisionEnabled` _staticmesh1 "NoCollision")
  (set `/Game/BluePrints/BP_Player.HandlingObject` self (`self.Player`))
  (`self.K2_SetActorRelativeRotation` (struct :`Pitch` 90.0))
  ;[1 1 1] 벽에 붙어있는 종이 > 줍게되면 물리 적용됨
  (`PrimitiveComponent.SetSimulatePhysics` (`self.StaticMesh1`) true))

(event `self.Inspect End`
  (params (BP_Player :type "/Game/BluePrints/BP_Player Object Reference"))
  (bind _staticmesh1 (`self.StaticMesh1`))
  (set `self.Player` BP_Player)
  (`self.DisableInput` (`GameplayStatics.GetPlayerController` 0))
  (`self.K2_SetActorRelativeLocation` (0.0 0.0 0.0))
  (`self.K2_DetachFromActor` "KeepWorld" "KeepWorld")
  (`PrimitiveComponent.SetSimulatePhysics` _staticmesh1 true)
  (`PrimitiveComponent.SetCollisionEnabled` _staticmesh1 "QueryAndPhysics"))

(fn `UserConstructionScript`)