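; Base actor for objects the player can pick up and inspect.
; InspectStart enables input, snaps the object to the player's Item component with physics and collision off, sets a fixed relative rotation and registers it as the player's HandlingObject.
; InspectEnd disables input, resets relative location, detaches and restores physics and collision.
; An unconnected node for placing the object in front of the camera never runs.
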(event `/Game/BluePrints/InspectInteract.Inspect Start`
  (params (BP_Player :type "/Game/BluePrints/BP_Player Object Reference"))
  (bind _inspectmesh (`self.InspectMesh`))
  (set `self.Player` BP_Player)
  (`self.EnableInput` (`GameplayStatics.GetPlayerController` 0))
  (`self.K2_AttachToComponent` (`/Game/BluePrints/BP_Player.Item` (`self.Player`)) "None" "SnapToTarget" "SnapToTarget" "KeepRelative")
  (`PrimitiveComponent.SetSimulatePhysics` _inspectmesh false)
  (`PrimitiveComponent.SetCollisionEnabled` _inspectmesh "NoCollision")
  (set `/Game/BluePrints/BP_Player.HandlingObject` self (`self.Player`))
  (`self.K2_SetActorRelativeRotation` (struct :`Pitch` 90.0)))

(event `/Game/BluePrints/InspectInteract.Inspect End`
  (params (BP_Player :type "/Game/BluePrints/BP_Player Object Reference"))
  (bind _inspectmesh (`self.InspectMesh`))
  (set `self.Player` BP_Player)
  (`self.DisableInput` (`GameplayStatics.GetPlayerController` 0))
  (`self.K2_SetActorRelativeLocation` (0.0 0.0 0.0))
  (`self.K2_DetachFromActor` "KeepWorld" "KeepWorld")
  (`PrimitiveComponent.SetSimulatePhysics` _inspectmesh true)
  (`PrimitiveComponent.SetCollisionEnabled` _inspectmesh "QueryAndPhysics"))

(fn `UserConstructionScript`)