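; BP_Locker is an interactable three-dial combination lock that the player zooms in on to open.
; Empty-hand interaction blends to the locker's camera and enables cursor input; Escape blends back to the player.
; Each left-click release joins the child BP_LockerDial numbers and compares them to PassWord as integers.
; A match plays a drawer timeline, then zooms out, destroys the actor and shows an unlock message; wrong-password feedback is unconnected.
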(event `self.ReceiveBeginPlay`
  (bind _dial (`self.Dial`))
  (bind _asbp_locker_dial (cast `/Game/BluePrints/BP_Locker/BP_LockerDial` (`ChildActorComponent.ChildActor` (`self.BP_LockerDial_1`))))
  (`KismetArrayLibrary.Array_Add` _dial _asbp_locker_dial)
  (bind _asbp_locker_dial_2 (cast `/Game/BluePrints/BP_Locker/BP_LockerDial` (`ChildActorComponent.ChildActor` (`self.BP_LockerDial_2`))))
  (`KismetArrayLibrary.Array_Add` _dial _asbp_locker_dial_2)
  (bind _asbp_locker_dial_3 (cast `/Game/BluePrints/BP_Locker/BP_LockerDial` (`ChildActorComponent.ChildActor` (`self.BP_LockerDial_3`))))
  (`KismetArrayLibrary.Array_Add` _dial _asbp_locker_dial_3))

(event `/Game/BluePrints/EmptyHandInterface.Empty Hand Interact`
  ;[1 1 1] Focus On Locker
  (`self.ZoomIn`)
  (`self.EnableInput` (`GameplayStatics.GetPlayerController` 0)))

(event `EnhancedInput|/Game/Inputs/IA_MouseLeftClick`
  (params (ActionValue :type Boolean) (ElapsedSeconds :type "Float (double-precision)") (TriggeredSeconds :type "Float (double-precision)") (InputAction :type "InputAction Object Reference" :default "/Game/Inputs/IA_MouseLeftClick.IA_MouseLeftClick"))
  (:`Completed`
    (set `self.DialWord` "")
    (for _array_element (`self.Dial`)
      (set `self.DialWord` (`KismetStringLibrary.Concat_StrStr` (`self.DialWord`) (`KismetStringLibrary.Conv_IntToString` (`/Game/BluePrints/BP_Locker/BP_LockerDial.DialNumber` _array_element)))))
    ;[1 1 1] 비밀번호 확인
    (`KismetSystemLibrary.PrintString` (`self.DialWord`))
    (if (== (`KismetStringLibrary.Conv_StringToInt` (`self.PassWord`)) (`KismetStringLibrary.Conv_StringToInt` (`self.DialWord`)))
      ;[1 1 1] 잠금해제 및 애니메이션
      (set `self.Locked` false)
      (bind (_direction _drawer) (`Timeline|타임라인`)
        (:`Update`
          (`SceneComponent.K2_SetRelativeLocation` (`self.StaticMesh1`) (`KismetMathLibrary.MakeVector` 0.0 0.0 _drawer) false false))
        (:`Finished`
          (`self.ZoomOut`)
          ;[1 1 1] 자물쇠 삭제
          (`self.K2_DestroyActor`)
          ;[1 1 1] 성공효과음
          (`GameplayStatics.PlaySoundAtLocation` "/Game/BluePrints/Sounds/Succesed__Cue.Succesed__Cue" (0.0 0.0 0.0) (struct) 1.0 1.0 0.0 null null null null)
          ;[1 1 1] 잠금이 해제되었습니다 메세지 출력
          (bind _returnvalue (`|CreateWidget` "/Game/BluePrints/UI_Notifications/UI_Message.UI_Message_C" (`GameplayStatics.GetPlayerController` 0)))
          (`/Game/BluePrints/UI_Notifications/UI_Message.Set Text` _returnvalue "잠금이 해제되었습니다.")
          (`UserWidget.AddToViewport` _returnvalue 0)
          (`KismetSystemLibrary.Delay` 2.0)
          (`Widget.RemoveFromParent` _returnvalue))))))

(event `Key|Escape`
  (params (Key :type "Key Structure"))
  ;[1 1 1] ESC : ZoomOut
  (:`Pressed`
    (`self.ZoomOut`)))

(event `ZoomOut`
  (bind _returnvalue (`GameplayStatics.GetPlayerController` 0))
  ;[1 1 1] 카메라 복원
  (bind _asbp_player (cast `/Game/BluePrints/BP_Player` (`GameplayStatics.GetPlayerCharacter` 0)))
  (`PlayerController.SetViewTargetWithBlend` (`GameplayStatics.GetPlayerController` 0) _asbp_player 0.4 "VTBlend_Linear" 0.0 false)
  ;[1 1 1] 커서 및 마우스 이벤트 비활성화
  (bind _output_get (set `PlayerController.bShowMouseCursor` false _returnvalue))
  (bind _output_get_2 (set `PlayerController.bEnableClickEvents` _output_get _returnvalue))
  (set `PlayerController.bEnableMouseOverEvents` _output_get_2 _returnvalue))

(event `ZoomIn`
  (bind _returnvalue (`GameplayStatics.GetPlayerController` 0))
  ;[1 1 1] ZoomIn동작
  (`PlayerController.SetViewTargetWithBlend` (`GameplayStatics.GetPlayerController` 0) (`ActorComponent.GetOwner` (`self.Camera`)) 0.4 "VTBlend_Linear" 0.0 false)
  ;[1 1 1] 커서 및 마우스 벤트 활성화
  (bind _output_get (set `PlayerController.bShowMouseCursor` true _returnvalue))
  (bind _output_get_2 (set `PlayerController.bEnableClickEvents` _output_get _returnvalue))
  (set `PlayerController.bEnableMouseOverEvents` _output_get_2 _returnvalue))

(fn `UserConstructionScript`)