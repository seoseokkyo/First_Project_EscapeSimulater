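; BP_RotateTest is a combination locker prototype that zooms the view onto three child-actor dials on empty-hand interaction.
; BeginPlay caches the dials; interacting blends to the locker camera and enables cursor, click and hover events, while Escape restores the player view.
; Unconnected logic compares joined dial digits to the password, then plays a sound, slides a mesh by timeline and destroys the actor.
; Result message widgets are also unconnected.
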(event `self.ReceiveBeginPlay`
  (bind _dial (`self.Dial`))
  ;[1 1 1] Dial들을 배열로 보관
  (bind _asbp_locker_dial (cast `/Game/BluePrints/BP_Locker/BP_LockerDial` (`ChildActorComponent.ChildActor` (`self.BP_LockerDial_1`))))
  (`KismetArrayLibrary.Array_Add` _dial _asbp_locker_dial)
  (bind _asbp_locker_dial_2 (cast `/Game/BluePrints/BP_Locker/BP_LockerDial` (`ChildActorComponent.ChildActor` (`self.BP_LockerDial_2`))))
  (`KismetArrayLibrary.Array_Add` _dial _asbp_locker_dial_2)
  (bind _asbp_locker_dial_3 (cast `/Game/BluePrints/BP_Locker/BP_LockerDial` (`ChildActorComponent.ChildActor` (`self.BP_LockerDial_3`))))
  (`KismetArrayLibrary.Array_Add` _dial _asbp_locker_dial_3))

(event `self.Empty Hand Interact`
  ;[1 1 1] Focus On Locker
  (`self.ZoomIn`)
  (`self.EnableInput` (`GameplayStatics.GetPlayerController` 0)))

(event `EnhancedInput|/Game/Inputs/IA_MouseLeftClick`
  (params (ActionValue :type Boolean) (ElapsedSeconds :type "Float (double-precision)") (TriggeredSeconds :type "Float (double-precision)") (InputAction :type "InputAction Object Reference" :default "/Game/Inputs/IA_MouseLeftClick.IA_MouseLeftClick")))

(event `Key|Escape`
  (params (Key :type "Key Structure"))
  ;[1 1 1] ESC : ZoomOut
  (:`Pressed`
    (`self.ZoomOut`)))

(event `ZoomOut`
  (bind _returnvalue (`GameplayStatics.GetPlayerController` 0))
  ;[1 1 1] 카메라 복원
  (bind _asbp_player (cast `/Game/BluePrints/BP_Player` (`GameplayStatics.GetPlayerCharacter` 0)))
  (`PlayerController.SetViewTargetWithBlend` (`GameplayStatics.GetPlayerController` 0) _asbp_player 0.4 "VTBlend_Linear" 0.0 false)
  ;[1 1 1] 커서 및 마우스 이벤트 비활성화
  (bind _output_get (set `PlayerController.bShowMouseCursor` false _returnvalue))
  (bind _output_get_2 (set `PlayerController.bEnableClickEvents` _output_get _returnvalue))
  (set `PlayerController.bEnableMouseOverEvents` _output_get_2 _returnvalue))

(event `ZoomIn`
  (bind _returnvalue (`GameplayStatics.GetPlayerController` 0))
  ;[1 1 1] ZoomIn동작
  (`PlayerController.SetViewTargetWithBlend` (`GameplayStatics.GetPlayerController` 0) (`ActorComponent.GetOwner` (`self.Camera`)) 0.4 "VTBlend_Linear" 0.0 false)
  ;[1 1 1] 커서 및 마우스 벤트 활성화
  (bind _output_get (set `PlayerController.bShowMouseCursor` true _returnvalue))
  (bind _output_get_2 (set `PlayerController.bEnableClickEvents` _output_get _returnvalue))
  (set `PlayerController.bEnableMouseOverEvents` _output_get_2 _returnvalue))

(fn `UserConstructionScript`)