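; First-person player Blueprint for an interaction game, handling movement, look, a quit menu and clockwork-key obtained/used popups.
; Tick line-traces from the camera to track the viewed actor, driving highlights and an interact-dot crosshair.
; Left click dispatches through interfaces to pick up, use, place or drop items; placed targets handle hand-state cleanup because placement can fail.
; Space toggles inspection of held items, centering them, freezing look and enabling cursor-driven rotation.
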(event `self.ReceiveBeginPlay`
  ;[1 1 1] Player Initialize
  (`|ExecutionSequence`
    (:`then_0`
      ;[1 1 1] 플레이어 조작 방식 맵핑
      (`EnhancedInputSubsystemInterface.AddMappingContext` (pcsubsystem `EnhancedInputLocalPlayerSubsystem` (`GameplayStatics.GetPlayerController` 0)) "/Game/Inputs/IA_Lovomotion.IA_Lovomotion" 0 (struct)))
    (:`then_1`
      ;[1 1 1] Interact 강조표시 (크로스헤어) 위젯 생성
      (bind _returnvalue (`|CreateWidget` "/Game/BluePrints/InteractDotWidget.InteractDotWidget_C"))
      (set `self.InteractDotWidget` _returnvalue))))

(event `EnhancedInput|/Game/Inputs/IA_MoveForward`
  (params (ActionValue :type "Float (double-precision)") (ElapsedSeconds :type "Float (double-precision)") (TriggeredSeconds :type "Float (double-precision)") (InputAction :type "InputAction Object Reference" :default "/Game/Inputs/IA_MoveForward.IA_MoveForward"))
  (bind (_returnvalue_roll _returnvalue_pitch _returnvalue_yaw) (`KismetMathLibrary.BreakRotator` (`self.GetControlRotation`)))
  ;[1 1 1] 앞뒤좌우 Move
  (:`Triggered`
    (`self.AddMovementInput` (`KismetMathLibrary.GetForwardVector` (`KismetMathLibrary.MakeRotator` 0.0 0.0 _returnvalue_yaw)) ActionValue)))

(event `EnhancedInput|/Game/Inputs/IA_MoveRight`
  (params (ActionValue :type "Float (double-precision)") (ElapsedSeconds :type "Float (double-precision)") (TriggeredSeconds :type "Float (double-precision)") (InputAction :type "InputAction Object Reference" :default "/Game/Inputs/IA_MoveRight.IA_MoveRight"))
  (bind (_returnvalue_roll _returnvalue_pitch _returnvalue_yaw) (`KismetMathLibrary.BreakRotator` (`self.GetControlRotation`)))
  ;[1 1 1] 앞뒤좌우 Move
  (:`Triggered`
    (`self.AddMovementInput` (`KismetMathLibrary.GetRightVector` (`KismetMathLibrary.MakeRotator` 0.0 0.0 _returnvalue_yaw)) ActionValue)))

(event `EnhancedInput|/Game/Inputs/IA_LookUp`
  (params (ActionValue :type "Float (double-precision)") (ElapsedSeconds :type "Float (double-precision)") (TriggeredSeconds :type "Float (double-precision)") (InputAction :type "InputAction Object Reference" :default "/Game/Inputs/IA_LookUp.IA_LookUp"))
  ;[1 1 1] 화면 회전(마우스로 시야 변경)
  (:`Triggered`
    (if (not (`self.CursorInteractOn`))
      (`self.AddControllerPitchInput` ActionValue))))

(event `EnhancedInput|/Game/Inputs/IA_LookRight`
  (params (ActionValue :type "Float (double-precision)") (ElapsedSeconds :type "Float (double-precision)") (TriggeredSeconds :type "Float (double-precision)") (InputAction :type "InputAction Object Reference" :default "/Game/Inputs/IA_LookRight.IA_LookRight"))
  ;[1 1 1] 화면 회전(마우스로 시야 변경)
  (:`Triggered`
    (if (not (`self.CursorInteractOn`))
      (`self.AddControllerYawInput` ActionValue))))

(event `Key|Escape`
  (params (Key :type "Key Structure"))
  (:`Pressed`
    (bind _output_get (set `self.showWindow` (xor (`self.showWindow`) true)))
    (if _output_get
      (bind _returnvalue (`|CreateWidget` "/Game/UI/UI_Quit.UI_Quit_C" (`GameplayStatics.GetPlayerController` 0)))
      (bind _output_get_2 (set `self.QuitUI` _returnvalue))
      (`UserWidget.AddToViewport` _output_get_2 0)
      (else
        (`Widget.RemoveFromParent` (`self.QuitUI`))
        (set `PlayerController.bShowMouseCursor` false (`GameplayStatics.GetPlayerController` 0))))))

(event `self.ReceiveTick`
  (params (DeltaSeconds :type "Float (single-precision)"))
  (bind _correctactor (`self.CorrectActor`))
  (bind _interactdotwidget (`self.InteractDotWidget`))
  (bind _returnvalue (`Widget.IsInViewport` (`self.InteractDotWidget`)))
  ;[1 1 1] 도트위젯 체크
  (`self.InteractDotWidget`
    (:`then`
      ;[1 1 1] 라인트레이스 기능 실행
      (bind _hitactor (`self.HitActor` 300.0))
      ;[1 1 1] Hit된 액터가 있는지 확인
      (`/Engine/EditorBlueprintResources/StandardMacros.IsValid` _hitactor
        (:`Is Valid`
          (if (== _hitactor (`self.CorrectActor`))
            (message `/Game/BluePrints/HighlightInterface.HighLightOn` _correctactor)
            (else
              (message `/Game/BluePrints/HighlightInterface.HighLightOff` _correctactor)))
          ;[1 1 1] Hit여부에 따라 보고있는 액터 저장
          (set `self.CorrectActor` _hitactor)
          ;[1 1 1] Hit된 액터가 Interact기능이 있는지 확인
          (if (`KismetSystemLibrary.DoesImplementInterface` _hitactor "/Game/BluePrints/InteractInterface.InteractInterface_C")
            ;[1 1 1] Hit된 액터가 Interact인터페이스가 있으면 크로스헤어 표시
            ; 또는 Hit되지 않거나 Interact인터페이스가 없을 경우 크로스헤어 삭제
            (if (not _returnvalue)
              (`UserWidget.AddToViewport` _interactdotwidget 0))
            (else
              (if _returnvalue :!label _label
                (`Widget.RemoveFromParent` _interactdotwidget)))))
        (:`Is Not Valid`
          (set `self.CorrectActor` null)
          (goto _label))))
    (:`else`)))

(event `InspStart`
  (bind _correctactor (`self.CorrectActor`))
  ;[1 1 1] Inspect인터페이스가 있는 경우 Inspect기능 실행
  (message `/Game/BluePrints/InspectInteract.Inspect Start` _correctactor self)
  (set `self.HandlingObject` _correctactor)
  (set `self.EmptyHand` false))

(event `EnhancedInput|/Game/Inputs/IA_MouseLeftClick`
  (params (ActionValue :type Boolean) (ElapsedSeconds :type "Float (double-precision)") (TriggeredSeconds :type "Float (double-precision)") (InputAction :type "InputAction Object Reference" :default "/Game/Inputs/IA_MouseLeftClick.IA_MouseLeftClick"))
  (bind _handlingobject (`self.HandlingObject`))
  (bind _correctactor (`self.CorrectActor`))
  (:`Completed`
    ;[1 1 1] 좌클릭이 입력된 시점에서 Player의 손이 비어있는지 확인
    (if (`self.CursorInteractOn`)
      _
      (elif (`self.EmptyHand`)
        ;[1 1 1] 보고있는 액터를 검증 후 Inspect인터페이스가 있는지 확인
        (`/Engine/EditorBlueprintResources/StandardMacros.IsValid` _correctactor
          (:`Is Valid`
            (if (`KismetSystemLibrary.DoesImplementInterface` _correctactor "/Game/BluePrints/InspectInteract.InspectInteract_C")
              (`self.InspStart`)
              (else
                ;[1 1 1] Empty Hand 인터페이스가 있는지 확인 후 Empty Hand Interact기능 실행
                (if (`KismetSystemLibrary.DoesImplementInterface` (`self.CorrectActor`) "/Game/BluePrints/EmptyHandInterface.EmptyHandInterface_C")
                  (message `/Game/BluePrints/EmptyHandInterface.Empty Hand Interact` (`self.CorrectActor`)))))))
        (else
          ;[1 1 1] 손에 들고있는 액터를 검증 후 보고있는 액터에 Place Interface가 있는지 확인 (액터, 플래그 정리는 내부에서 진행)
          ; 여기서 플레이어의 손에 든 액터 및 플래그를 정리하지 않는 이유는 Place라는 행동을 실패할 수 있기 때문.
          (`/Engine/EditorBlueprintResources/StandardMacros.IsValid` (`self.HandlingObject`)
            (:`Is Valid`
              (if (`KismetSystemLibrary.DoesImplementInterface` (`self.CorrectActor`) "/Game/BluePrints/PlaceInterface.PlaceInterface_C")
                (message `/Game/BluePrints/PlaceInterface.PlaceInteract` (`self.CorrectActor`) (`self.HandlingObject`))
                (else
                  ;[1 1 1] Inspect인터페이스가 있는 경우 해당 액터를 땅에 버림 (플레이어의 손에서 떨어지는 동작은 내부에서 진행됨)
                  (`/Engine/EditorBlueprintResources/StandardMacros.IsValid` _handlingobject
                    (:`Is Valid`
                      (if (`KismetSystemLibrary.DoesImplementInterface` _handlingobject "/Game/BluePrints/InspectInteract.InspectInteract_C")
                        (message `/Game/BluePrints/InspectInteract.Inspect End` _handlingobject self)
                        (set `self.EmptyHand` true)))))))))))))

(event `Key|SpaceBar`
  (params (Key :type "Key Structure"))
  (:`Pressed`
    (`self.ToggleCursorInteract`)))

(event `ToggleCursorInteract`
  (bind _returnvalue (`GameplayStatics.GetPlayerController` 0))
  (bind _returnvalue_2 (`GameplayStatics.GetPlayerController` 0))
  (bind _handlingobject (`self.HandlingObject`))
  (bind _handlingobject_2 (`self.HandlingObject`))
  (if (not (`self.EmptyHand`))
    (bind _output_get (set `self.CursorInteractOn` (xor (`self.CursorInteractOn`) true)))
    (if _output_get
      (`SceneComponent.K2_SetRelativeLocation` (`self.ItemPosition`) (63.0 -0.0 0.0) false false)
      (if (`KismetSystemLibrary.DoesImplementInterface` _handlingobject "/Game/BluePrints/InspectInteract.InspectInteract_C")
        (message `/Game/BluePrints/InspectInteract.Rotate On` _handlingobject)
        (bind _output_get_2 (set `PlayerController.bShowMouseCursor` true _returnvalue))
        (bind _output_get_3 (set `PlayerController.bEnableClickEvents` _output_get_2 _returnvalue))
        (set `PlayerController.bEnableMouseOverEvents` _output_get_3 _returnvalue))
      (else
        (`SceneComponent.K2_SetRelativeLocation` (`self.ItemPosition`) (96.666667 23.333 -16.66666) false false)
        (if (`KismetSystemLibrary.DoesImplementInterface` _handlingobject_2 "/Game/BluePrints/InspectInteract.InspectInteract_C")
          (message `/Game/BluePrints/InspectInteract.RotateOff` _handlingobject_2)
          (bind _output_get_4 (set `PlayerController.bShowMouseCursor` false _returnvalue_2))
          (bind _output_get_5 (set `PlayerController.bEnableClickEvents` _output_get_4 _returnvalue_2))
          (set `PlayerController.bEnableMouseOverEvents` _output_get_5 _returnvalue_2))))))

(event `InsideHaveHandle`
  (params (HaveHandle :type Boolean))
  (bind _output_get (set `self.haveHandle` HaveHandle))
  (if _output_get
    ;[1 1 1] Message 팝업 (태엽을 획득했습니다.)
    (bind _returnvalue (`|CreateWidget` "/Game/BluePrints/UI_Notifications/UI_Message.UI_Message_C"))
    (`UserWidget.AddToViewport` _returnvalue 0)
    (`/Game/BluePrints/UI_Notifications/UI_Message.Set Text` _returnvalue "태엽을 획득했습니다.")
    (`KismetSystemLibrary.Delay` 2.0)
    (`Widget.RemoveFromParent` _returnvalue)
    (else
      ;[1 1 1] Message 팝업 (태엽을 사용하였습니다.)
      (bind _returnvalue_2 (`|CreateWidget` "/Game/BluePrints/UI_Notifications/UI_Message.UI_Message_C"))
      (`UserWidget.AddToViewport` _returnvalue_2 0)
      (`/Game/BluePrints/UI_Notifications/UI_Message.Set Text` _returnvalue_2 "태엽을 사용하였습니다.")
      (`KismetSystemLibrary.Delay` 2.0)
      (`Widget.RemoveFromParent` _returnvalue_2))))

(fn `Call Toggle Cursor`
  (`self.ToggleCursorInteract`)
  (return))

(fn `CallInspStart`
  (`self.InspStart`)
  (return))

(fn `HitActor`
  (params (InteractDistance :type "Float (double-precision)"))
  (returns (HitActor :type "Actor Object Reference"))
  (bind _camera (`self.Camera`))
  (bind _returnvalue (`SceneComponent.K2_GetComponentLocation` _camera))
  ;[1 1 1] 카메라의 정면방향에서 Interact Distance까지의 액터를 찾음
  (bind (_outhit _returnvalue_2) (`KismetSystemLibrary.LineTraceSingle` _returnvalue (+ _returnvalue (* (`SceneComponent.GetForwardVector` _camera) InteractDistance)) "TraceTypeQuery1"))
  ;[1 1 1] 카메라가 보는 방향의 Interact Distance거리에 액터가 있을 시 반환
  ; 액터가 없을 시 nullptr 반환
  (if _returnvalue_2
    (return (`.HitActor` (`GameplayStatics.BreakHitResult` _outhit)))
    (else
      (return null))))

(fn `SetHaveHandle`
  (params (HaveHandle :type Boolean))
  (`self.InsideHaveHandle` HaveHandle)
  (return))

(fn `UserConstructionScript`)