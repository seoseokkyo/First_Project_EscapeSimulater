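; Interactable strongbox puzzle that opens when a three-digit code matches its password.
; Empty-hand interaction blends to the box camera with cursor and click events, and Escape returns to the player.
; BeginPlay labels ten child-actor buttons and makes the BP_DoorKey mesh visible.
; AddNumber fills three child-actor dials in turn and checks the code, then chained timelines move the camera, turn the handle, zoom out and swing the door.
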(event `self.ReceiveBeginPlay`
  (`self.CreateStrongBox`)
  (bind _returnvalue (`GameplayStatics.GetActorOfClass` "/Game/BluePrints/BP_Door/BP_DoorKey.BP_DoorKey_C"))
  (`SceneComponent.SetVisibility` (`/Game/BluePrints/BP_Door/BP_DoorKey.Door_Key` _returnvalue) true false))

(event `/Game/BluePrints/EmptyHandInterface.Empty Hand Interact`
  ;[1 1 1] Focus On Locker
  (`self.ZoomIn`)
  (`self.EnableInput` (`GameplayStatics.GetPlayerController` 0)))

(event `Key|Escape`
  (params (Key :type "Key Structure"))
  ;[1 1 1] ESC : ZoomOut
  (:`Pressed`
    (`self.ZoomOut`)))

(event `ZoomOut`
  (bind _returnvalue (`GameplayStatics.GetPlayerController` 0))
  ;[1 1 1] 카메라 복원
  (bind _asbp_player (cast `/Game/BluePrints/BP_Player` (`GameplayStatics.GetPlayerCharacter` 0)))
  (`PlayerController.SetViewTargetWithBlend` (`GameplayStatics.GetPlayerController` 0) _asbp_player 0.4 "VTBlend_Linear" 0.0 false)
  ;[1 1 1] 커서 및 마우스 이벤트 비활성화
  (bind _output_get (set `PlayerController.bShowMouseCursor` false _returnvalue))
  (bind _output_get_2 (set `PlayerController.bEnableClickEvents` _output_get _returnvalue))
  (set `PlayerController.bEnableMouseOverEvents` _output_get_2 _returnvalue))

(event `ZoomIn`
  (bind _returnvalue (`GameplayStatics.GetPlayerController` 0))
  ;[1 1 1] ZoomIn동작
  (if (not (`self.Opened`))
    (`PlayerController.SetViewTargetWithBlend` (`GameplayStatics.GetPlayerController` 0) (`ActorComponent.GetOwner` (`self.Camera`)) 0.4 "VTBlend_Linear" 0.0 false)
    ;[1 1 1] 커서 및 마우스 벤트 활성화
    (bind _output_get (set `PlayerController.bShowMouseCursor` true _returnvalue))
    (bind _output_get_2 (set `PlayerController.bEnableClickEvents` _output_get _returnvalue))
    (set `PlayerController.bEnableMouseOverEvents` _output_get_2 _returnvalue)))

(event `Open`
  ;[1 1 1] ZoomOut 및 다시 ZoomIn이 되는것을 막을 플래그
  (set `self.Opened` true)
  ;[1 1 1] 핸들 Rotate
  (bind (_direction _newtrack_0) (`Timeline|Timeline_1`)
    (:`Update`
      (`SceneComponent.K2_SetRelativeLocation` (`self.Camera`) (`KismetMathLibrary.MakeVector` 55.0 15.0 (+ _newtrack_0 44.6)) false false))
    (:`Finished`
      (bind (_direction_2 _newtrack_0_2) (`Timeline|Timeline_0`)
        (:`Update`
          (`SceneComponent.K2_SetRelativeRotation` (`self.Front_Handle`) (`KismetMathLibrary.MakeRotator` 0.0 _newtrack_0_2) false false))
        (:`Finished`
          (`self.ZoomOut`)
          ;[1 1 1] Door Open
          (bind (_direction_3 _newtrack_2) (`Timeline|Timeline`)
            (:`Update`
              (`SceneComponent.K2_SetRelativeRotation` (`self.Front_DoorAndPanel`) (`KismetMathLibrary.MakeRotator` 0.0 0.0 _newtrack_2) false false))))))))

(fn `AddNumber`
  (params (InputNumber :type String))
  (returns (Complete :type Boolean))
  (bind _returnvalue (`KismetStringLibrary.Conv_StringToInt` InputNumber))
  ;[1 1 1] 3개의 다이얼 및 비밀번호를 컨트롤하기 위함
  (if (>= (`self.InputCount`) 3)
    (set `self.InputCount` 0)
    (set `self.CurrentNumber` ""))
  ;[1 1 1] 맞는 다이얼을 찾고, 찾은 다이얼의 숫자를 보여주는 구간
  (bind _output_get (set `self.CurrentNumber` (`KismetStringLibrary.Concat_StrStr` (`self.CurrentNumber`) InputNumber)))
  (`KismetSystemLibrary.PrintString` _output_get)
  (if (== (`self.InputCount`) 0)
    (bind _asbp_strong_box_dial (cast `/Game/BluePrints/BP_StrongBox/BP_StrongBoxDial` (`ChildActorComponent.ChildActor` (`self.BP_StrongBoxDial_1`))))
    (`/Game/BluePrints/BP_StrongBox/BP_StrongBoxDial.SetNumber` _asbp_strong_box_dial _returnvalue)
    (bind _result (`/Engine/EditorBlueprintResources/StandardMacros.IncrementInt` (`self.InputCount`) :!label _label)
      (:`  `
        (set `self.InputCount` _result)
        (bind _equal (`self.CheckPassword`))
        (if _equal
          (`self.Open`)
          (return true)
          (else
            (return false)))))
    (elif (== (`self.InputCount`) 1)
      (bind _asbp_strong_box_dial_2 (cast `/Game/BluePrints/BP_StrongBox/BP_StrongBoxDial` (`ChildActorComponent.ChildActor` (`self.BP_StrongBoxDial_2`))))
      (`/Game/BluePrints/BP_StrongBox/BP_StrongBoxDial.SetNumber` _asbp_strong_box_dial_2 _returnvalue)
      (goto _label)
      (elif (== (`self.InputCount`) 2)
        (bind _asbp_strong_box_dial_3 (cast `/Game/BluePrints/BP_StrongBox/BP_StrongBoxDial` (`ChildActorComponent.ChildActor` (`self.BP_StrongBoxDial_3`))))
        (`/Game/BluePrints/BP_StrongBox/BP_StrongBoxDial.SetNumber` _asbp_strong_box_dial_3 _returnvalue)
        (goto _label)))))

(fn `CheckPassword`
  (returns (Equal :type Boolean))
  (return (== (`KismetStringLibrary.Conv_StringToInt` (`self.Password`)) (`KismetStringLibrary.Conv_StringToInt` (`self.CurrentNumber`)))))

(fn `CreateStrongBox`
  ;[1 1 1] 버튼Initial 및 배열생성구간
  (bind _output_get (set `self.ButtonArray` (`|MakeArray` (`self.BP_StrongBoxButton_0`) (`self.BP_StrongBoxButton_1`) (`self.BP_StrongBoxButton_2`) (`self.BP_StrongBoxButton_3`) (`self.BP_StrongBoxButton_4`) (`self.BP_StrongBoxButton_5`) (`self.BP_StrongBoxButton_6`) (`self.BP_StrongBoxButton_7`) (`self.BP_StrongBoxButton_8`) (`self.BP_StrongBoxButton_9`))))
  (for (_array_element _array_index) _output_get
    (bind _asbp_strong_box_button (cast `/Game/BluePrints/BP_StrongBox/BP_StrongBoxButton` (`ChildActorComponent.ChildActor` _array_element)))
    (`/Game/BluePrints/BP_StrongBox/BP_StrongBoxButton.SetText` _asbp_strong_box_button (`KismetStringLibrary.Conv_IntToString` _array_index))))

(fn `UserConstructionScript`)