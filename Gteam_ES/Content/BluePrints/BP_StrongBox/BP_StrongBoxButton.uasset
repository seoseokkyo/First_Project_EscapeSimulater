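; BP_StrongBoxButton is a pressable number button that sits as a child actor on a BP_StrongBox.
; On release, a Push timeline plays, then the button sends its text to the parent strongbox via AddNumber, plays a press sound and runs a Release timeline.
; SetText and GetText manage the value shown on its text render component and passed to the box.
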(event `self.StrongBoxButton.OnReleased`
  (params (TouchedComponent :type "PrimitiveComponent Object Reference") (ButtonReleased :type "Key Structure"))
  (`Timeline|Push`
    (:`Finished`
      (bind _asbp_strong_box (cast `/Game/BluePrints/BP_StrongBox/BP_StrongBox` (`self.GetParentActor`)))
      (`/Game/BluePrints/BP_StrongBox/BP_StrongBox.AddNumber` _asbp_strong_box (`self.Text`))
      (`GameplayStatics.PlaySoundAtLocation` "/Game/BluePrints/Sounds/StrongBox/ButtonPress_Cue.ButtonPress_Cue" (0.0 0.0 0.0) (struct) 1.0 1.0 0.0 null null null null)
      (`Timeline|Release`))))

(fn `GetText`
  (returns (NewParam :type String))
  (return (`self.Text`)))

(fn `SetText`
  (params (Text :type String))
  (bind _output_get (set `self.Text` Text))
  (`TextRenderComponent.K2_SetText` (`self.TextRender`) (`KismetTextLibrary.Conv_StringToText` _output_get)))

(fn `UserConstructionScript`)