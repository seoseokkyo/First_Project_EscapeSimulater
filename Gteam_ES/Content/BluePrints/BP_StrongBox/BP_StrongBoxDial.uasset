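; Strongbox dial actor that shows a digit from 0 to 9 by its rotation, in 36-degree steps.
; SetNumber snaps the relative yaw to the given digit without updating DialNumber, which BeginPlay resets to zero.
; The click event is empty.
; Unconnected leftovers hold a timeline-animated advance with sound and a loop-based pitch rotation toward a target number, neither of which runs.
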(event `self.ReceiveBeginPlay`
  (set `self.DialNumber` 0))

(event `self.StaticMesh.OnClicked`
  (params (TouchedComponent :type "PrimitiveComponent Object Reference") (ButtonPressed :type "Key Structure")))

(fn `SetNumber`
  (params (InputNumber :type Integer))
  (`self.K2_SetActorRelativeRotation` (`KismetMathLibrary.MakeRotator` 0.0 0.0 (`KismetMathLibrary.Conv_IntToDouble` (* InputNumber 36)))))

(fn `UserConstructionScript`)