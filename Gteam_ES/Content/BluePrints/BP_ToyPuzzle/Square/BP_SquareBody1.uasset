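; Toy puzzle body that accepts the square puzzle piece the player is holding.
; On PlaceInteract it casts the incoming actor to BP_SquarePuzzle, ignoring anything else, then sets IsSquare and reveals its own BPSquarePuzzle to show the piece inserted.
; It then empties the player's hand state on BP_Player and destroys the held piece, so placement is a visibility swap rather than an attachment.
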(event `self.PlaceInteract`
  (params (TryInteractActor :type "Actor Object Reference"))
  ;[1 1 1] 상호작용 하는 퍼즐이 Square 퍼즐이 맞는지 확인 > 맞을시 Is Square : True
  (bind _asbp_square_puzzle (cast `/Game/BluePrints/BP_ToyPuzzle/Square/BP_SquarePuzzle` TryInteractActor))
  (set `self.As BP Square Puzzle` _asbp_square_puzzle)
  (set `self.Is Square` true)
  ;[1 1 1] 맞으면 Body 에 퍼즐 끼워진 상태로 상태 변함
  (`SceneComponent.SetVisibility` (`self.BP_SquarePuzzle`) true false)
  ;[1 1 1] 손에 든 퍼즐 사라짐
  (bind _asbp_player (cast `/Game/BluePrints/BP_Player` (`GameplayStatics.GetPlayerCharacter` 0)))
  (set `/Game/BluePrints/BP_Player.EmptyHand` true _asbp_player)
  (set `/Game/BluePrints/BP_Player.HandlingObject` null _asbp_player)
  (`self.K2_DestroyActor` (`self.As BP Square Puzzle`)))

(fn `UserConstructionScript`)