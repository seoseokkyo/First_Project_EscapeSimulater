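; BP_SquarePuzzle is a box puzzle toy that the player can pick up to inspect and put down.
; InspectStart snaps it to the player's ItemPosition, turns off Square's physics and collision, and rotates the actor to face the view.
; InspectEnd detaches it and restores physics and collision.
; Both highlight events set Square's custom depth rendering to false, so HighLighton shows no outline.
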(event `/Game/BluePrints/InspectInteract.Inspect Start`
  (params (BP_Player :type "/Game/BluePrints/BP_Player Object Reference"))
  (bind _square (`self.Square`))
  ;[1 1 1] 상자퍼즐을 플레이어 시야에 붙임
  (set `self.player` BP_Player)
  (`self.K2_AttachToComponent` (`/Game/BluePrints/BP_Player.ItemPosition` (`self.player`)) "None" "SnapToTarget" "SnapToTarget" "KeepRelative")
  ;[1 1 1] 피직스 시뮬레이트를 끄고 콜리전 설정을 변경함
  (`SceneComponent.K2_SetRelativeLocation` _square (0.0 0.0 0.0) false false)
  (`PrimitiveComponent.SetSimulatePhysics` _square false)
  (`PrimitiveComponent.SetCollisionEnabled` _square "NoCollision")
  ;[1 1 1] self의 각도를 변경
  (`self.K2_SetActorRelativeRotation` (struct :`Pitch` 90.0)))

(event `/Game/BluePrints/HighlightInterface.HighLightOn`
  (`PrimitiveComponent.SetRenderCustomDepth` (`self.Square`) false))

(event `/Game/BluePrints/InspectInteract.Inspect End`
  (params (BP_Player :type "/Game/BluePrints/BP_Player Object Reference"))
  (bind _square (`self.Square`))
  ;[1 1 1] 퍼즐을 놓음
  (set `self.player` BP_Player)
  (`SceneComponent.K2_SetRelativeLocation` (`self.Square`) (0.0 0.0 0.0) false false)
  (`self.K2_DetachFromActor` "KeepWorld" "KeepWorld")
  ;[1 1 1] 피직스 시뮬레이트를 키고 콜리전 설정을 변경함
  (`PrimitiveComponent.SetSimulatePhysics` _square true)
  (`PrimitiveComponent.SetCollisionEnabled` _square "QueryAndPhysics"))

(event `/Game/BluePrints/HighlightInterface.HighLightOff`
  (`PrimitiveComponent.SetRenderCustomDepth` (`self.Square`) false))

(fn `UserConstructionScript`)