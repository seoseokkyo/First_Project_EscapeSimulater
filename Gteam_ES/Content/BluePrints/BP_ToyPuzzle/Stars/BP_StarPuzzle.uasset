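; BP_StarPuzzle is a toy puzzle object the player can pick up, inspect in view and drop.
; InspectStart enables input, snaps it to the player's ItemPosition, rotates it and disables the Cube's physics and collision.
; InspectEnd disables input, detaches it and restores physics and collision.
; Both highlight events switch the Cube's custom depth rendering off, so neither shows a highlight.
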(event `self.Inspect Start`
  (params (BP_Player :type "/Game/BluePrints/BP_Player Object Reference"))
  (bind _cube (`self.Cube`))
  ;[1 1 1] 상자퍼즐을 플레이어 시야에 붙임
  (set `self.player` BP_Player)
  (`self.EnableInput` (`GameplayStatics.GetPlayerController` 0))
  (`self.K2_AttachToComponent` (`/Game/BluePrints/BP_Player.ItemPosition` (`self.player`)) "None" "SnapToTarget" "SnapToTarget" "KeepRelative")
  ;[1 1 1] 피직스 시뮬레이트를 끄고 콜리전 설정을 변경함
  (`SceneComponent.K2_SetRelativeLocation` _cube (0.0 0.0 0.0) false false)
  (`PrimitiveComponent.SetSimulatePhysics` _cube false)
  (`PrimitiveComponent.SetCollisionEnabled` _cube "NoCollision")
  ;[1 1 1] self의 각도를 변경
  (`self.K2_SetActorRelativeRotation` (struct :`Pitch` 90.0)))

(event `self.HighLightOn`
  (`PrimitiveComponent.SetRenderCustomDepth` (`self.Cube`) false))

(event `self.Inspect End`
  (params (BP_Player :type "/Game/BluePrints/BP_Player Object Reference"))
  (bind _cube (`self.Cube`))
  ;[1 1 1] 퍼즐을 놓음
  (set `self.player` BP_Player)
  (`self.DisableInput` (`GameplayStatics.GetPlayerController` 0))
  (`SceneComponent.K2_SetRelativeLocation` (`self.Cube`) (0.0 0.0 0.0) false false)
  (`self.K2_DetachFromActor` "KeepWorld" "KeepWorld")
  ;[1 1 1] 피직스 시뮬레이트를 키고 콜리전 설정을 변경함
  (`PrimitiveComponent.SetSimulatePhysics` _cube true)
  (`PrimitiveComponent.SetCollisionEnabled` _cube "QueryAndPhysics"))

(event `self.HighLightOff`
  (`PrimitiveComponent.SetRenderCustomDepth` (`self.Cube`) false))

(fn `UserConstructionScript`)