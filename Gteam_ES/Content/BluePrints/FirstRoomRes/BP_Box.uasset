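; BP_Box is an interactable box with a hinged lid that can be secured by a child-actor BP_Locker.
; BeginPlay caches the locker; empty-hand interaction shows a two-second "box is locked" UI_Message in Korean while it is locked.
; Without a valid or locked locker, interaction plays a sound at world origin and runs a Timeline forward or reverse to rotate BoxHead.
; A State flag blocks retriggering mid-animation, and Open flips on finish.
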(event `self.ReceiveBeginPlay`
  ;[1 1 1] 자식 컴퍼넌트 액터 클래스인 Locker를 액터 클래스 형태로 보관
  (bind _asbp_locker (cast `/Game/BluePrints/BP_Locker/BP_Locker` (`ChildActorComponent.ChildActor` (`self.BP_Locker`))))
  (set `self.BP Locker` _asbp_locker))

(event `/Game/BluePrints/EmptyHandInterface.Empty Hand Interact`
  (bind _bp_locker (`self.BP Locker`))
  ;[1 1 1] 자물쇠가 Valid한 상태인지 검증 및 잠금상태 체크
  (`/Engine/EditorBlueprintResources/StandardMacros.IsValid` _bp_locker
    (:`Is Valid`
      (if (`/Game/BluePrints/BP_Locker/BP_Locker.Locked` _bp_locker)
        ;[1 1 1] 퍼즐을 풀었습니다! UI 출력
        (bind _returnvalue (`|CreateWidget` "/Game/BluePrints/UI_Notifications/UI_Message.UI_Message_C" (`GameplayStatics.GetPlayerController` 0)))
        (`/Game/BluePrints/UI_Notifications/UI_Message.Set Text` _returnvalue "상자가 잠겨있습니다.")
        (`UserWidget.AddToViewport` _returnvalue 0)
        (`KismetSystemLibrary.Delay` 2.0)
        (`Widget.RemoveFromParent` _returnvalue)
        (else
          ;[1 1 1] Animation 중복 실행 방지를 위한 플래그 체크 및 Box의 Open, Close체크
          (if (`self.State`) :!label _label
            (`GameplayStatics.PlaySoundAtLocation` "/Game/BluePrints/Sounds/DoorOpen_Cue.DoorOpen_Cue" (0.0 0.0 0.0) (struct) 1.0 1.0 0.0 null null null null)
            (if (`self.Open`)
              (set `self.State` false)
              ;[1 1 1] Box Open Close Animation
              (bind (_direction _drawer) (`Timeline|Timeline` :!label _label_2)
                (:`Update`
                  (`SceneComponent.K2_SetRelativeRotation` (`self.BoxHead`) (`KismetMathLibrary.MakeRotator` 0.0 _drawer) false false))
                (:`Finished`
                  ;[1 1 1] 플래그 관리
                  (set `self.State` true)
                  (set `self.Open` (xor (`self.Open`) true))))
              (else
                (set `self.State` false)
                (goto _label_2 :!via `Reverse`)))))))
    (:`Is Not Valid`
      (goto _label))))

(fn `UserConstructionScript`)