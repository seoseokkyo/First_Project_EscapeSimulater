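; BP_DeskSlot is an interactable desk drawer that slides between two positions when EmptyHandInteract is called.
; A timeline's Drawer track drives the relative Y location of the SMDesk component, playing forward or in reverse according to the Open flag.
; The AnimationEnd flag blocks interaction mid-slide, and the timeline's Finished output re-enables it and toggles Open.
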(event `/Game/BluePrints/EmptyHandInterface.Empty Hand Interact`
  (if (`self.animationEnd`)
    (if (`self.Open`)
      (set `self.animationEnd` false)
      (bind (_direction _drawer) (`Timeline|Timeline` :!label _label)
        (:`Update`
          (`SceneComponent.K2_SetRelativeLocation` (`self.SM_Desk`) (`KismetMathLibrary.MakeVector` 0.0 _drawer) false false))
        (:`Finished`
          (set `self.animationEnd` true)
          (set `self.Open` (xor (`self.Open`) true))))
      (else
        (set `self.animationEnd` false)
        (goto _label :!via `Reverse`)))))

(fn `UserConstructionScript`)