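; BP_Window is an interactable window that slides vertically open and closed when the EmptyHandInteract event fires.
; A timeline drives the relative Z location of the WindowTheresaA component, playing forward or in reverse depending on the Open flag.
; A State flag blocks new interactions during the animation, and the timeline's Finished output re-enables it and toggles Open.
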(event `/Game/BluePrints/EmptyHandInterface.Empty Hand Interact`
  ;[1 1 1] Animation 중복실행 방지를 위한 상태체크 및 Open Close체크
  (if (`self.State`)
    (if (`self.Open`)
      (set `self.State` false)
      ;[1 1 1] Window Open Close Animation
      (bind (_direction _drawer) (`Timeline|Timeline` :!label _label)
        (:`Update`
          (`SceneComponent.K2_SetRelativeLocation` (`self.WindowTheresa_a`) (`KismetMathLibrary.MakeVector` 0.0 0.0 _drawer) false false))
        (:`Finished`
          ;[1 1 1] 플래그 관리
          (set `self.State` true)
          (set `self.Open` (xor (`self.Open`) true))))
      (else
        (set `self.State` false)
        (goto _label :!via `Reverse`)))))

(fn `UserConstructionScript`)