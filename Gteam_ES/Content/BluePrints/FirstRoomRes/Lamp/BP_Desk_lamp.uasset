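; Desk lamp Blueprint for the first room that reveals a password when switched on.
; LightToggle flips LightState and calls LightOn or LightOff, which set the spotlight intensity and show or clear the hard-coded code on a TextRender.
; The password starts blank at BeginPlay.
; The EmptyHandInteract event is empty, and nothing in this Blueprint calls LightToggle.
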(event `self.ReceiveBeginPlay`
  (bind _output_get (set `self.Password` ""))
  (`TextRenderComponent.K2_SetText` (`self.TextRender`) _output_get))

(event `/Game/BluePrints/EmptyHandInterface.Empty Hand Interact`)

(fn `LightOff`
  (`LightComponent.SetIntensity` (`self.SpotLight`) 0.0)
  (bind _output_get (set `self.Password` ""))
  (`TextRenderComponent.K2_SetText` (`self.TextRender`) _output_get))

(fn `LightOn`
  (`LightComponent.SetIntensity` (`self.SpotLight`) 10000.0)
  (bind _output_get (set `self.Password` "389"))
  (`TextRenderComponent.K2_SetText` (`self.TextRender`) _output_get))

(fn `LightToggle`
  (if (xor (`self.LightState`) true)
    (`self.LightOn`)
    (set `self.LightState` true)
    (else
      (`self.LightOff`)
      (set `self.LightState` false))))

(fn `UserConstructionScript`)