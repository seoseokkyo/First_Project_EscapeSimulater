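; BP_Desk_lamp_Switch is the desk lamp's interactable switch, toggled by empty-hand interaction.
; A State flag plays or reverses a timeline that pitches the switch mesh, with an AnimationEnd flag meant to block overlapping animations.
; When the timeline finishes, it flips State, calls LightToggle on the parent BP_Desk_lamp actor and plays the lamp sound.
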(event `/Game/BluePrints/EmptyHandInterface.Empty Hand Interact`
  ;[1 1 1] Animation 중복실행 방지를 위한 상태체크 및 Open Close체크
  (if (`self.Animation End`)
    (if (`self.State`)
      (set `self.Animation End` false)
      ;[1 1 1] 서랍 Animation
      (bind (_direction _switching) (`Timeline|타임라인` :!label _label)
        (:`Update`
          (`SceneComponent.K2_SetRelativeRotation` (`self.StaticMesh`) (`KismetMathLibrary.MakeRotator` 0.0 _switching) false false))
        (:`Finished`
          ;[1 1 1] 플래그 관리
          (set `self.Animation End` true)
          (set `self.State` (xor (`self.State`) true))
          (bind _asbp_desk_lamp (cast `/Game/BluePrints/FirstRoomRes/Lamp/BP_Desk_lamp` (`self.GetParentActor`)))
          (`/Game/BluePrints/FirstRoomRes/Lamp/BP_Desk_lamp.LightToggle` _asbp_desk_lamp)
          (`GameplayStatics.PlaySoundAtLocation` "/Game/BluePrints/Sounds/LampOn_Cue.LampOn_Cue" (0.0 0.0 0.0) (struct) 1.0 1.0 0.0 null null null null)))
      (else
        (set `self.Animation End` (`self.Animation End`))
        (goto _label :!via `Reverse`)))))

(fn `UserConstructionScript`)