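; BP_Wardrobe is a first-room wardrobe actor that carries a BP_Locker as a child actor and reports whether it is locked.
; On BeginPlay it casts the child actor to BP_Locker and caches the reference.
; CheckLockerState copies that locker's Locked flag into its own Locked variable and returns it, treating an invalid locker as unlocked.
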(event `self.ReceiveBeginPlay`
  ;[1 1 1] 자식 컴퍼넌트 형태의 액터 클래스를 액터 클래스 형태로 변환하여 보관
  (bind _asbp_locker (cast `/Game/BluePrints/BP_Locker/BP_Locker` (`ChildActorComponent.ChildActor` (`self.BP_Locker`))))
  (set `self.BP Locker` _asbp_locker))

(fn `CheckLockerState`
  (returns (State :type Boolean))
  (bind _bp_locker (`self.BP Locker`))
  ;[1 1 1] Locker의 상태를 체크
  (`/Engine/EditorBlueprintResources/StandardMacros.IsValid` _bp_locker
    (:`Is Valid`
      (if (`/Game/BluePrints/BP_Locker/BP_Locker.Locked` _bp_locker)
        (bind _output_get (set `self.Locked` true))
        (return _output_get)
        (else
          (bind _output_get_2 (set `self.Locked` false))
          (return _output_get_2))))
    (:`Is Not Valid`
      (bind _output_get_3 (set `self.Locked` false))
      (return _output_get_3))))

(fn `UserConstructionScript`)