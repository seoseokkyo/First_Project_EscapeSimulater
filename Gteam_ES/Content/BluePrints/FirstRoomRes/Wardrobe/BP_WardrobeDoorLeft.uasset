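; Left door of the first-room wardrobe, which swings open and closed on empty-hand interaction.
; It asks its parent BP_Wardrobe whether it is locked and, if so, shows a two-second "locked" message in Korean.
; Otherwise it plays a sound and runs a timeline forward or in reverse to set door yaw, flipping State on finish.
; The AnimationEnd flag blocks repeat triggers, but is only cleared on forward play.
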(event `/Game/BluePrints/EmptyHandInterface.Empty Hand Interact`
  (bind _asbp_wardrobe (cast `/Game/BluePrints/FirstRoomRes/Wardrobe/BP_Wardrobe` (`self.GetParentActor`)))
  (bind _state (`/Game/BluePrints/FirstRoomRes/Wardrobe/BP_Wardrobe.CheckLockerState` _asbp_wardrobe))
  (if _state
    ;[1 1 1] 잠겨있습니다. 메세지 출력
    (bind _returnvalue (`|CreateWidget` "/Game/BluePrints/UI_Notifications/UI_Message.UI_Message_C" (`GameplayStatics.GetPlayerController` 0)))
    (`/Game/BluePrints/UI_Notifications/UI_Message.Set Text` _returnvalue "잠겨있습니다.")
    (`UserWidget.AddToViewport` _returnvalue 0)
    (`KismetSystemLibrary.Delay` 2.0)
    (`Widget.RemoveFromParent` _returnvalue)
    (else
      ;[1 1 1] Animation 중복실행 방지를 위한 상태체크 및 Open Close체크
      (if (`self.Animation End`)
        (`GameplayStatics.PlaySoundAtLocation` "/Game/BluePrints/Sounds/Drawer_Cue.Drawer_Cue" (0.0 0.0 0.0) (struct) 1.0 1.0 0.0 null null null null)
        (if (`self.State`)
          (set `self.Animation End` false)
          ;[1 1 1] 서랍 Animation
          (bind (_direction _switching) (`Timeline|타임라인` :!label _label)
            (:`Update`
              (`SceneComponent.K2_SetRelativeRotation` (`self.WardrobeDoor_b_left`) (`KismetMathLibrary.MakeRotator` 0.0 0.0 _switching) false false))
            (:`Finished`
              ;[1 1 1] 플래그 관리
              (set `self.Animation End` true)
              (set `self.State` (xor (`self.State`) true))))
          (else
            (set `self.Animation End` (`self.Animation End`))
            (goto _label :!via `Reverse`)))))))

(fn `UserConstructionScript`)