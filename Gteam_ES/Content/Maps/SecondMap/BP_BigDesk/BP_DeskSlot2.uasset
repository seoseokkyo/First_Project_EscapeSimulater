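; BP_DeskSlot2 is a desk drawer in SecondMap that slides open or closed on an empty-hand interaction.
; A timeline drives the SMDesk mesh's relative Y position, playing forward or in reverse according to the Open flag.
; AnimationEnd blocks re-triggering mid-motion, and both flags update when the timeline finishes.
; Drawer_Cue plays at the world origin on interaction and on every timeline update.
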(event `self.Empty Hand Interact`
  ;[1 1 1] Animation 중복실행 방지를 위한 상태체크 및 Open Close체크
  (if (`self.animationEnd`)
    (`GameplayStatics.PlaySoundAtLocation` "/Game/BluePrints/Sounds/Drawer_Cue.Drawer_Cue" (0.0 0.0 0.0) (struct) 1.0 1.0 0.0 null null null null)
    (if (`self.Open`)
      (set `self.animationEnd` false)
      ;[1 1 1] 서랍 Animation
      (bind (_direction _drawer) (`Timeline|Timeline` :!label _label)
        (:`Update`
          (`GameplayStatics.PlaySoundAtLocation` "/Game/BluePrints/Sounds/Drawer_Cue.Drawer_Cue" (0.0 0.0 0.0) (struct) 1.0 1.0 0.0 null null null null)
          (`SceneComponent.K2_SetRelativeLocation` (`self.SM_Desk`) (`KismetMathLibrary.MakeVector` 0.0 _drawer) false false))
        (:`Finished`
          ;[1 1 1] 플래그 관리
          (set `self.animationEnd` true)
          (set `self.Open` (xor (`self.Open`) true))))
      (else
        (set `self.animationEnd` false)
        (goto _label :!via `Reverse`)))))

(fn `UserConstructionScript`)