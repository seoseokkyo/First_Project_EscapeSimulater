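; Puzzle board actor where the player places BP_PuzzleChunk pieces into a 4x4 grid to solve a puzzle.
; BeginPlay builds scene-component slots with parallel state structs, then spawns locked pieces into the InitialChunkNumber slots.
; PlaceInteract snaps a held piece to the slot given by its own PlacedNumber if free, and empties the player's hand.
; After each placement it checks all slots and sets TargetSolved1 on BP_GameState when full.
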(event `self.ReceiveBeginPlay`
  (`self.CreatePuzzleBoard` 16)
  (for _array_element (`self.PuzzleDataArray`)
    (for _array_element_2 (`self.InitialChunkNumber`)
      (bind (_bplaced _placednumber) (break `/Game/Puzzle/T_PuzzleData` _array_element))
      (if (== _array_element_2 _placednumber)
        (bind _output (`|GetArrayItem` (`self.ComponentArray`) _placednumber))
        (bind _returnvalue (`|SpawnActorFromClass` "/Game/Puzzle/BP_PuzzleChunk.BP_PuzzleChunk_C" (`KismetMathLibrary.MakeTransform` (`SceneComponent.K2_GetComponentLocation` _output) (struct) (0.2 0.2 0.5)) "Undefined" "MultiplyWithRoot" null null))
        (`self.K2_AttachToComponent` _returnvalue _output "None" "SnapToTarget" "SnapToTarget" "KeepRelative" true)
        (bind _inspectmesh (`/Game/BluePrints/BP_InspectParent.InspectMesh` _returnvalue))
        (`PrimitiveComponent.SetSimulatePhysics` _inspectmesh false)
        (`PrimitiveComponent.SetCollisionEnabled` _inspectmesh "NoCollision")
        (`self.SetActorScale3D` _returnvalue (0.2 0.2 0.05))
        (bind (_returnvalue_x _returnvalue_y _returnvalue_z) (`KismetMathLibrary.BreakVector` (`SceneComponent.K2_GetComponentLocation` _output)))
        (`self.K2_SetActorLocation` _returnvalue (`KismetMathLibrary.MakeVector` _returnvalue_x _returnvalue_y (- _returnvalue_z 4.0)) false false)
        (`self.DisableInput` _returnvalue (`GameplayStatics.GetPlayerController` 0))
        (`KismetArrayLibrary.Array_Set` (`self.PuzzleDataArray`) _placednumber (make `/Game/Puzzle/T_PuzzleData` true _placednumber _returnvalue))))))

(event `/Game/BluePrints/PlaceInterface.PlaceInteract`
  (params (TryInteractActor :type "Actor Object Reference"))
  (bind _inputchunkindex (`self.InputChunkIndex`))
  (bind (_returnvalue_x _returnvalue_y _returnvalue_z) (`KismetMathLibrary.BreakVector` (`SceneComponent.K2_GetComponentLocation` (`self.FoundedScene`))))
  (bind (_returnvalue_roll _returnvalue_pitch _returnvalue_yaw) (`KismetMathLibrary.BreakRotator` (`SceneComponent.K2_GetComponentRotation` (`self.FoundedScene`))))
  ;[1 1 1] 퍼즐조각인지 확인
  (bind _asbp_puzzle_chunk (cast `/Game/Puzzle/BP_PuzzleChunk` TryInteractActor)
    (:`then`
      ;[1 1 1] 들어온 퍼즐이 위치할 자리가 비어있는지 확인
      (bind _output_get (set `self.InputChunk` _asbp_puzzle_chunk))
      (bind (_puzzlechunkdata_bplaced _puzzlechunkdata_placednumber) (break `/Game/Puzzle/T_PuzzleData` (`/Game/Puzzle/BP_PuzzleChunk.PuzzleChunkData` _output_get)))
      (bind (_output_bplaced _output_placednumber) (break `/Game/Puzzle/T_PuzzleData` (`|GetArrayItem` (`self.PuzzleDataArray`) _puzzlechunkdata_placednumber)))
      (set `self.InputChunkIndex` _output_placednumber)
      (if (== _output_bplaced false)
        ;[1 1 1] PuzzleData Array 갱신
        (`KismetArrayLibrary.Array_Set` (`self.PuzzleDataArray`) _inputchunkindex (make `/Game/Puzzle/T_PuzzleData` true _inputchunkindex (`self.InputChunk`)))
        ;[1 1 1] 들어온 퍼즐조각의 위치 검색
        (for (_array_element _array_index) (`self.ComponentArray`)
          (if (== _array_index (`self.InputChunkIndex`))
            (set `self.FoundedScene` _array_element)
            ;[1 1 1] 플레이어 손의 퍼즐조각을 때어냄
            (`self.K2_DetachFromActor` (`self.InputChunk`) "KeepWorld" "KeepWorld" "KeepRelative")
            ;[1 1 1] Comment
            (`self.K2_AttachToComponent` (`self.FoundedScene`) "None" "SnapToTarget" "SnapToTarget" "KeepRelative")
            ;[1 1 1] 퍼즐조각의 위치를 검색된 SceneComponent로 이동시킴
            (`self.K2_SetActorLocation` (`self.InputChunk`) (`KismetMathLibrary.MakeVector` _returnvalue_x _returnvalue_y (- _returnvalue_z 4.0)) false false)
            ;[1 1 1] 퍼즐조각의 회전을 검색된 SceneComponent의 회전값으로 변경
            (`self.K2_SetActorRelativeRotation` (`self.InputChunk`) (`KismetMathLibrary.MakeRotator` _returnvalue_roll _returnvalue_pitch _returnvalue_yaw) false false)
            ;[1 1 1] 플레이어의 손에 아무것도 없는 상태로 변경
            (bind _asbp_player (cast `/Game/BluePrints/BP_Player` (`GameplayStatics.GetPlayerCharacter` 0)))
            (set `/Game/BluePrints/BP_Player.EmptyHand` true _asbp_player)
            ;[1 1 1] 퍼즐보드에 퍼즐이 놓일 때 마다 퍼즐의 완성을 체크
            ; 퍼즐이 완성된 경우 GameState에 알림
            (set `self.EndCheck` true)
            (for _array_element_2 (`self.PuzzleDataArray`)
              (bind _output_get_2 (set `self.EndCheck` (== (`.bPlaced_1_9D3853524E597C9B60A16C866851ADB2` (break `/Game/Puzzle/T_PuzzleData` _array_element_2)) true)))
              (if (not _output_get_2)
                (break)))
            (if (`self.EndCheck`)
              (`KismetSystemLibrary.PrintString` "All Puzzle Completed!" true true (struct :`G` 0.66 :`B` 1.0 :`A` 1.0) 10.0)
              (bind _asbp_game_state (cast `/Game/BluePrints/BP_GameState` (`GameplayStatics.GetGameState`)))
              (set `/Game/BluePrints/BP_GameState.TargetSolved_1` true _asbp_game_state))))
        (else
          ;[1 1 1] 해당 위치에 이미 퍼즐이 있는 경우
          (bind _asbp_player_2 (cast `/Game/BluePrints/BP_Player` (`GameplayStatics.GetPlayerCharacter` 0)))
          (set `/Game/BluePrints/BP_Player.EmptyHand` false _asbp_player_2))))
    (:`CastFailed`
      (`KismetSystemLibrary.PrintString` "CastFailed"))))

(fn `CreatePuzzleBoard`
  (params (NumberChunk :type Integer))
  ;[1 1 1] Number To Index
  (for _index (range NumberChunk)
    ;[1 1 1] 각 위치에 Scene Component 배치
    (bind _returnvalue (`AddComponent|NODE_AddSceneComponent-3` :`RelativeTransform` (`KismetMathLibrary.MakeTransform` (`KismetMathLibrary.MakeVector` (`KismetMathLibrary.Conv_IntToDouble` (+ (* (/ _index 4) 20) (`self.ChunkPosX`))) (`KismetMathLibrary.Conv_IntToDouble` (+ (* (mod _index 4) 20) (`self.ChunkPosY`))) 4.0))))
    ;[1 1 1] Scene Component 배열보관
    (`KismetArrayLibrary.Array_Add` (`self.ComponentArray`) _returnvalue)
    ;[1 1 1] 각 슬롯들의 상태를 확인하는 구조체 보관
    (`KismetArrayLibrary.Array_Add` (`self.PuzzleDataArray`) (make `/Game/Puzzle/T_PuzzleData` false _index null))))

(fn `UserConstructionScript`)